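; Player controller for the spaceship path map, where the player advances node by node and spends resources on event choices.
; Loads map, resources and cursor from BP_GameInstance, spawns BP_PathMap and its widget, and saves on EndPlay.
; Completed nodes unlock cursor moves along connections; affordable choices deduct costs and show random outcomes, or roll credits at the last column.
; Resource changes trigger the fuel detour to m_planet or crew/food game-over.
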(event `ModifyResource`
  (params (Resource :type "/Game/BP/Events/Resourcen Enum" :default "NewEnumerator0") (Value :type Integer))
  (for (_array_element _array_index) (`self.Resources`)
    (if (`|EnumEquality` (break `/Game/BP/Pathmap/PlayerResources` _array_element) Resource)
      (`KismetArrayLibrary.Array_Set` (`self.Resources`) _array_index (make `/Game/BP/Pathmap/PlayerResources` (break `/Game/BP/Pathmap/PlayerResources` _array_element) (`KismetMathLibrary.Clamp` (+ (`.Amount_5_7811A45048D81ACB18AD8785644683AF` (break `/Game/BP/Pathmap/PlayerResources` _array_element)) Value) (`KismetMathLibrary.SelectInt` 1 0 (`|EnumEquality` (break `/Game/BP/Pathmap/PlayerResources` _array_element) "NewEnumerator0")) 999) (`.Icon_8_63A8BBCA4B5882340FF227B42F64F577` (break `/Game/BP/Pathmap/PlayerResources` _array_element))))
      (bind (_output_resource _output_amount) (break `/Game/BP/Pathmap/PlayerResources` (`|GetArrayItem` (`self.Resources`) _array_index)))
      (`self.OnResourceChanged` (break `/Game/BP/Pathmap/PlayerResources` _array_element) _output_amount (`.Amount_5_7811A45048D81ACB18AD8785644683AF` (break `/Game/BP/Pathmap/PlayerResources` _array_element))))))

(event `self.ReceiveEndPlay`
  (params (EndPlayReason :type "EEndPlayReason Enum" :default "Destroyed"))
  (`self.SaveState`))

(event `SaveState`
  (bind _asbp_game_instance (cast `/Game/Core/BP_GameInstance` (`GameplayStatics.GetGameInstance`)))
  (`/Game/Core/BP_GameInstance.SaveState` _asbp_game_instance (`self.Resources`) (`self.CursorX`) (`self.CursorY`)))

(event `self.ReceiveBeginPlay`
  (bind _asbp_game_instance (cast `/Game/Core/BP_GameInstance` (`GameplayStatics.GetGameInstance`)))
  (set `self.MaxHeight` (`/Game/Core/BP_GameInstance.MapHeight` _asbp_game_instance))
  (set `self.MaxWidth` (`/Game/Core/BP_GameInstance.MapWidth` _asbp_game_instance))
  (set `self.Resources` (`/Game/Core/BP_GameInstance.Resources` _asbp_game_instance))
  (add `self.OnResourceChanged` (delegate `OnResourceChanged_Event_0`))
  (bind _returnvalue (`|SpawnActorFromClass` "/Game/BP/Pathmap/BP_PathMap.BP_PathMap_C" (`KismetMathLibrary.MakeTransform` (0.0 0.0 0.0)) "Undefined" "OverrideRootScale" null (`self.MaxWidth`) (`self.MaxHeight`) null))
  (set `self.PathMap` _returnvalue)
  (`WidgetBlueprintLibrary.SetInputMode_GameOnly` self)
  (bind _returnvalue_2 (`|CreateWidget` "/Game/BP/Pathmap/BP_PathMapWidget.BP_PathMapWidget_C"))
  (bind _output_get (set `self.UI_Widget` _returnvalue_2))
  (`UserWidget.AddToViewport` _output_get 0)
  (bind _asbp_game_instance_2 (cast `/Game/Core/BP_GameInstance` (`GameplayStatics.GetGameInstance`)))
  (set `self.RandomStream` (`KismetMathLibrary.MakeRandomStream` (`/Game/Core/BP_GameInstance.RandomSeed` _asbp_game_instance_2)))
  (set `self.CursorX` (`/Game/Core/BP_GameInstance.PlayerX` _asbp_game_instance_2))
  (bind _output_get_2 (set `self.CursorY` (`/Game/Core/BP_GameInstance.PlayerY` _asbp_game_instance_2)))
  (`/Game/BP/Pathmap/BP_PathMap.SetCursor` (`self.PathMap`) (`self.CursorX`) _output_get_2)
  (`self.OnCursorChange` (`self.CursorX`) (`self.CursorY`))
  (`/Game/BP/Pathmap/BP_PathMapWidget.Enable Choices` (`self.UI_Widget`)))

(event `Key|O`
  (params (Key :type "Key Structure"))
  (:`Pressed`
    (bind _returnvalue (`|CreateWidget` "/Game/BP/Pathmap/BP_Message.BP_Message_C" self "You ran out of fuel. But there is an asteroid belt nearby. Maybe you can find some glowing fuel orbs there." :!label _label))
    (add `/Game/BP/Pathmap/BP_Message.OnWidgetClosed` _returnvalue (delegate `OnWidgetClosed_Event_0`))
    (`UserWidget.AddToViewport` _returnvalue 0)))

(event `OnResourceChanged_Event_0` :!signature `self.OnResourceChanged`
  (params (Resource :type "/Game/BP/Events/Resourcen Enum" :default "NewEnumerator0") (NewAmount :type Integer) (ChangedBy :type Integer))
  (switch `/Game/BP/Events/Resourcen` Resource
    (:`NewEnumerator1`
      (if (<= NewAmount 0)
        (goto _label)))
    (:`NewEnumerator2`
      (if (<= NewAmount 0)
        (bind _returnvalue (`|CreateWidget` "/Game/BP/Pathmap/BP_Message.BP_Message_C" self "There no crew members left to operate this spacecraft. You lose."))
        (add `/Game/BP/Pathmap/BP_Message.OnWidgetClosed` _returnvalue (delegate `NoPersons`))
        (`UserWidget.AddToViewport` _returnvalue 0)))
    (:`NewEnumerator4`
      (if (<= NewAmount 0)
        (bind _returnvalue_2 (`|CreateWidget` "/Game/BP/Pathmap/BP_Message.BP_Message_C" self "You have no food left. All your crewmember starved. You lose."))
        (add `/Game/BP/Pathmap/BP_Message.OnWidgetClosed` _returnvalue_2 (delegate `StarvLose`))
        (`UserWidget.AddToViewport` _returnvalue_2 0)))))

(event `self.ReceiveTick`
  (params (DeltaSeconds :type "Float (single-precision)"))
  (`/Engine/EditorBlueprintResources/StandardMacros.IsValid` (`self.K2_GetPawn`)
    (:`Is Valid`
      (`/Engine/EditorBlueprintResources/StandardMacros.DoOnce` false
        (:`Completed`
          (`self.K2_SetActorLocation` (`self.PathMap`) (- (* (`KismetMathLibrary.GetForwardVector` (`self.GetControlRotation`)) 1000.0) (`KismetMathLibrary.MakeVector` (/ (* (`self.MaxWidth`) 256.0) 2.0) 500.0 (/ (* (`self.MaxHeight`) 256.0) 2.0))) false false))))))

(event `InputAxis|MoveForward`
  (params (AxisValue :type "Float (single-precision)"))
  (if (> AxisValue 0.0)
    (`/Engine/EditorBlueprintResources/StandardMacros.DoOnce` false :!label _label_2
      (:`Completed`
        (bind _return (`/Game/BP/Pathmap/Array2D.Get` (`/Game/BP/Pathmap/BP_PathMap.Array2D` (`self.PathMap`)) (`self.CursorX`) (`self.CursorY`)))
        (if (`.Done_14_2849FC10467D5C8A58602495B3439F55` (break `/Game/BP/Pathmap/PathPoint` _return))
          (bind _output_get (set `self.CursorY` (`KismetMathLibrary.Clamp` (+ (`self.CursorY`) 1) 0 (`self.MaxHeight`))))
          (if (`KismetArrayLibrary.Array_Contains` (`.Connections_8_B0926BA84A318D6543E413ACE86B1E9C` (break `/Game/BP/Pathmap/PathPoint` _return)) (make `/Game/BP/Pathmap/PathConnection` (`KismetMathLibrary.Clamp` (+ (`self.CursorX`) 1) 0 (`self.MaxWidth`)) _output_get))
            (set `self.CursorX` (`KismetMathLibrary.Clamp` (+ (`self.CursorX`) 1) 0 (`self.MaxWidth`)))
            (`/Game/BP/Pathmap/BP_PathMap.SetCursor` (`self.PathMap`) (`self.CursorX`) (`self.CursorY`) :!label _label_3)
            (`self.OnCursorChange` (`self.CursorX`) (`self.CursorY`))
            (`/Game/BP/Pathmap/BP_PathMapWidget.Enable Choices` (`self.UI_Widget`))
            (else
              (set `self.CursorY` (`KismetMathLibrary.Clamp` (- (`self.CursorY`) 1) 0 (`self.MaxHeight`))))))))
    (elif (< AxisValue 0.0)
      (`/Engine/EditorBlueprintResources/StandardMacros.DoOnce` false :!label _label_4
        (:`Completed`
          (bind _return_2 (`/Game/BP/Pathmap/Array2D.Get` (`/Game/BP/Pathmap/BP_PathMap.Array2D` (`self.PathMap`)) (`self.CursorX`) (`self.CursorY`)))
          (if (`.Done_14_2849FC10467D5C8A58602495B3439F55` (break `/Game/BP/Pathmap/PathPoint` _return_2))
            (bind _output_get_2 (set `self.CursorY` (`KismetMathLibrary.Clamp` (- (`self.CursorY`) 1) 0 (`self.MaxHeight`))))
            (if (`KismetArrayLibrary.Array_Contains` (`.Connections_8_B0926BA84A318D6543E413ACE86B1E9C` (break `/Game/BP/Pathmap/PathPoint` _return_2)) (make `/Game/BP/Pathmap/PathConnection` (`KismetMathLibrary.Clamp` (+ (`self.CursorX`) 1) 0 (`self.MaxWidth`)) _output_get_2))
              (set `self.CursorX` (`KismetMathLibrary.Clamp` (+ (`self.CursorX`) 1) 0 (`self.MaxWidth`)))
              (goto _label_3)
              (else
                (set `self.CursorY` (`KismetMathLibrary.Clamp` (+ (`self.CursorY`) 1) 0 (`self.MaxHeight`))))))))
      (else
        (`|ExecutionSequence`
          (:`then_0`
            (goto _label_2 :!via `Reset`))
          (:`then_1`
            (goto _label_4 :!via `Reset`)))))))

(event `OnWidgetClosed_Event_0`
  (`self.SaveState`)
  (`GameplayStatics.OpenLevel` "m_planet"))

(event `TranslateToUI`
  (params (`Axis Value` :type "Float (double-precision)"))
  (bind _ui_widget (`self.UI_Widget`))
  (if (!= `Axis Value` 0.0)
    (if (> `Axis Value` 0.0)
      (`/Game/BP/Pathmap/BP_PathMapWidget.Cursor Right` _ui_widget)
      (else
        (`/Game/BP/Pathmap/BP_PathMapWidget.Cursor Left` _ui_widget)))))

(event `NoPersons`
  (bind _asbp_game_instance (cast `/Game/Core/BP_GameInstance` (`GameplayStatics.GetGameInstance`)))
  (`/Game/Core/BP_GameInstance.StartNewGame` _asbp_game_instance)
  (`GameplayStatics.OpenLevel` "Overview"))

(event `Key|Enter`
  (params (Key :type "Key Structure"))
  (:`Pressed`
    (bind _return (`/Game/BP/Pathmap/Array2D.Get` (`/Game/BP/Pathmap/BP_PathMap.Array2D` (`self.PathMap`)) (`self.CursorX`) (`self.CursorY`)))
    (if (not (`.Done_14_2849FC10467D5C8A58602495B3439F55` (break `/Game/BP/Pathmap/PathPoint` _return)))
      (`/Game/BP/Pathmap/BP_PathMapWidget.Choose` (`self.UI_Widget`)))))

(event `InputAxis|MoveRight` :paused true
  (params (AxisValue :type "Float (single-precision)"))
  (`self.TranslateToUI` AxisValue)
  (if (< AxisValue 0.0)
    (`/Engine/EditorBlueprintResources/StandardMacros.DoOnce` false :!label _label_5
      (:`Completed`
        (bind _return (`/Game/BP/Pathmap/Array2D.Get` (`/Game/BP/Pathmap/BP_PathMap.Array2D` (`self.PathMap`)) (`self.CursorX`) (`self.CursorY`)))
        (if (`.Done_14_2849FC10467D5C8A58602495B3439F55` (break `/Game/BP/Pathmap/PathPoint` _return))
          (bind _output_get (set `self.CursorX` (`KismetMathLibrary.Clamp` (+ (`self.CursorX`) 1) 0 (`self.MaxWidth`))))
          (if (`KismetArrayLibrary.Array_Contains` (`.Connections_8_B0926BA84A318D6543E413ACE86B1E9C` (break `/Game/BP/Pathmap/PathPoint` _return)) (make `/Game/BP/Pathmap/PathConnection` _output_get (`self.CursorY`)))
            (goto _label_3)
            (else
              (set `self.CursorY` (`KismetMathLibrary.Clamp` (- (`self.CursorY`) 1) 0 (`self.MaxHeight`))))))))
    (else
      (goto _label_5 :!via `Reset`))))

(event `StarvLose`
  (bind _asbp_game_instance (cast `/Game/Core/BP_GameInstance` (`GameplayStatics.GetGameInstance`)))
  (`/Game/Core/BP_GameInstance.StartNewGame` _asbp_game_instance)
  (`GameplayStatics.OpenLevel` "Overview"))

(event `TryChoice`
  (params (Decision :type "/Game/BP/Events/EventDecision Structure"))
  (bind (_text _outcomes _requirements) (break `/Game/BP/Events/EventDecision` Decision))
  (bind _ui_widget (`self.UI_Widget`))
  (bind _cursorx (`self.CursorX`))
  (bind _result (`self.HasMaterials` Decision))
  (if _result
    (for _array_element _requirements
      (`self.ModifyResource` (`.Resource_5_B8290C3D47105D117F0D63BB4A88B92A` (break `/Game/BP/Events/EventOutcomeRequirement` _array_element)) (* (break `/Game/BP/Events/EventOutcomeRequirement` _array_element) -1)))
    (`GameplayStatics.PlaySound2D` "/Game/Sounds/confirm.confirm" 1.0 1.0 0.0 null null)
    (`/Game/BP/Pathmap/Array2D.SetDone` (`/Game/BP/Pathmap/BP_PathMap.Array2D` (`self.PathMap`)) (`self.CursorX`) (`self.CursorY`) true)
    (bind _return (`/Game/BP/Pathmap/Array2D.Get` (`/Game/BP/Pathmap/BP_PathMap.Array2D` (`self.PathMap`)) _cursorx (`self.CursorY`)))
    (if (and (== (`self.MaxWidth`) _cursorx) (`.Done_14_2849FC10467D5C8A58602495B3439F55` (break `/Game/BP/Pathmap/PathPoint` _return)))
      (`GameplayStatics.OpenLevel` "credits")
      (else
        (`/Game/BP/Pathmap/BP_PathMapWidget.Disable Choices` _ui_widget)
        (`/Game/BP/Pathmap/BP_PathMapWidget.ShowOutcome` _ui_widget (`|GetArrayItem` _outcomes (`KismetMathLibrary.RandomInteger` (- (`KismetArrayLibrary.Array_Length` _outcomes) 1))))))
    (else
      (`GameplayStatics.PlaySound2D` "/Game/Sounds/error.error" 1.0 1.0 0.0 null null))))

(fn `GetResource`
  (params (Res :type "/Game/BP/Events/Resourcen Enum" :default "NewEnumerator0"))
  (returns (PlayerRes :type "/Game/BP/Pathmap/PlayerResources Structure"))
  (for _array_element (`self.Resources`)
    (if (`|EnumEquality` Res (break `/Game/BP/Pathmap/PlayerResources` _array_element))
      (return (make `/Game/BP/Pathmap/PlayerResources` (break `/Game/BP/Pathmap/PlayerResources` _array_element) (`.Amount_5_7811A45048D81ACB18AD8785644683AF` (break `/Game/BP/Pathmap/PlayerResources` _array_element)) (`.Icon_8_63A8BBCA4B5882340FF227B42F64F577` (break `/Game/BP/Pathmap/PlayerResources` _array_element)))))))

(fn `HasMaterials`
  (params (Decision :type "/Game/BP/Events/EventDecision Structure"))
  (returns (Result :type Boolean))
  (locals (Res :type Boolean :default true))
  (for _array_element Decision_Requirements_11_D74BE5ED4C821939CA3F0D969105C4B8
    (bind _playerres (`self.GetResource` (`.Resource_5_B8290C3D47105D117F0D63BB4A88B92A` (break `/Game/BP/Events/EventOutcomeRequirement` _array_element))))
    (if (not (>= (`.Amount_5_7811A45048D81ACB18AD8785644683AF` (break `/Game/BP/Pathmap/PlayerResources` _playerres)) (break `/Game/BP/Events/EventOutcomeRequirement` _array_element)))
      (set `local.Res` false)))
  (return (`local.Res`)))

(fn `UserConstructionScript`)