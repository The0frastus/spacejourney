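; Grid-based path map that displays planet-type nodes as sprites, linked by route planes, with a cursor on the selected cell.
; BeginPlay seeds a random stream from BP_GameInstance, creates the Array2D grid and spawns a sprite per cell by type.
; UpdatePath destroys and rebuilds every connection mesh, tinting routes from the current cell differently.
; Tick calls SetCursor, so the cursor moves and all routes rebuild every frame.
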(event `self.ReceiveBeginPlay`
  (bind _maxwidth (`self.MaxWidth`))
  (bind _maxheight (`self.MaxHeight`))
  (bind _asbp_game_instance (cast `/Game/Core/BP_GameInstance` (`GameplayStatics.GetGameInstance`)))
  (set `self.RandomStream` (`KismetMathLibrary.MakeRandomStream` (`/Game/Core/BP_GameInstance.RandomSeed` _asbp_game_instance)))
  (`/Game/BP/Pathmap/Array2D.New` (`self.Array2D`) _maxheight _maxwidth)
  (for _index (range (+ _maxheight 1))
    (bind _output_get (set `self.Z` _index))
    (for _index_2 (range (+ _maxwidth 1))
      (bind _output_get_2 (set `self.X` _index_2))
      (bind _returnvalue (`AddComponent|NODE_AddPaperSpriteComponent-3` :`RelativeTransform` (`KismetMathLibrary.MakeTransform` (`KismetMathLibrary.MakeVector` (* _output_get_2 256.0) 0.0 (* _output_get 256.0)) (struct) (0.25 0.25 0.25))))
      (bind _return (`/Game/BP/Pathmap/Array2D.Get` (`self.Array2D`) (`self.X`) (`self.Z`)))
      (bind _output_get_3 (set `self.Connections` (`.Connections_8_B0926BA84A318D6543E413ACE86B1E9C` (break `/Game/BP/Pathmap/PathPoint` _return))))
      (`|ExecutionSequence`
        (:`then_0`
          (switch `/Game/BP/Pathmap/PointType` (break `/Game/BP/Pathmap/PathPoint` _return)
            (:`NewEnumerator0`
              (`PaperSpriteComponent.SetSprite` _returnvalue "/Game/Sprites/Planets/S_Wasser.S_Wasser"))
            (:`NewEnumerator1`
              (`PaperSpriteComponent.SetSprite` _returnvalue "/Game/Sprites/Planets/S_Feuer.S_Feuer"))
            (:`NewEnumerator2`
              (`PaperSpriteComponent.SetSprite` _returnvalue "/Game/Sprites/Planets/S_Ast.S_Ast"))
            (:`NewEnumerator3`
              (`PaperSpriteComponent.SetSprite` _returnvalue "/Game/Sprites/Planets/S_Erde.S_Erde"))
            (:`NewEnumerator4`
              (`PaperSpriteComponent.SetSprite` _returnvalue "/Game/Sprites/Planets/S_Gas.S_Gas"))))))
    (`self.UpdatePath` 0)))

(event `self.ReceiveTick`
  (params (DeltaSeconds :type "Float (single-precision)"))
  (bind (_selected_x _selected_y) (break `/Game/BP/Pathmap/PathConnection` (`self.Selected`)))
  (`self.SetCursor` _selected_x _selected_y))

(fn `SetCursor`
  (params (X :type Integer) (Y :type Integer))
  (bind _output_get (set `self.Selected` (make `/Game/BP/Pathmap/PathConnection` X Y)))
  (`SceneComponent.K2_SetRelativeLocation` (`self.PaperSprite`) (`KismetMathLibrary.MakeVector` (* (break `/Game/BP/Pathmap/PathConnection` _output_get) 256.0) 5.0 (* (`.Y_5_BB0787A0485E1E685404B7AEC90DC9AE` (break `/Game/BP/Pathmap/PathConnection` _output_get)) 256.0)) false false)
  (`self.UpdatePath` (break `/Game/BP/Pathmap/PathConnection` _output_get) (`.Y_5_BB0787A0485E1E685404B7AEC90DC9AE` (break `/Game/BP/Pathmap/PathConnection` _output_get))))

(fn `UpdatePath`
  (params (CurrentX :type Integer) (CurrentY :type Integer))
  (locals (Z :type Integer) (X :type Integer) (Connections :type "Array of /Game/BP/Pathmap/PathConnection Structure") (LocalCurrentX :type Integer) (LocalCurrentY :type Integer))
  (bind _returnvalue (`KismetMathLibrary.MakeVector` (* (`local.X`) 256.0) 0.0 (* (`local.Z`) 256.0)))
  (set `local.LocalCurrentX` CurrentX)
  (set `local.LocalCurrentY` CurrentY)
  (for _array_element (`self.Pathes`)
    (`/Engine/EditorBlueprintResources/StandardMacros.IsValid` _array_element
      (:`Is Valid`
        (`ActorComponent.K2_DestroyComponent` _array_element))))
  (`KismetArrayLibrary.Array_Clear` (`self.Pathes`))
  (for _index (range (+ (`self.MaxHeight`) 1))
    (set `local.Z` _index)
    (for _index_2 (range (+ (`self.MaxWidth`) 1))
      (set `local.X` _index_2)
      (bind _return (`/Game/BP/Pathmap/Array2D.Get` (`self.Array2D`) (`local.X`) (`local.Z`)))
      (bind _output_get (set `local.Connections` (`.Connections_8_B0926BA84A318D6543E413ACE86B1E9C` (break `/Game/BP/Pathmap/PathPoint` _return))))
      (if (> (`KismetArrayLibrary.Array_Length` _output_get) 0)
        (for _array_element_2 (`local.Connections`)
          (bind _returnvalue_2 (`KismetMathLibrary.MakeVector` (* (break `/Game/BP/Pathmap/PathConnection` _array_element_2) 256.0) 0.0 (* (`.Y_5_BB0787A0485E1E685404B7AEC90DC9AE` (break `/Game/BP/Pathmap/PathConnection` _array_element_2)) 256.0)))
          (bind _returnvalue_3 (- _returnvalue_2 _returnvalue))
          (bind _returnvalue_4 (`AddComponent|NODE_AddStaticMeshComponent-1` :`RelativeTransform` (`KismetMathLibrary.MakeTransform` (+ (/ _returnvalue_3 2.0) _returnvalue (0.0 -10.0 0.0)) (`KismetMathLibrary.ComposeRotators` (`KismetMathLibrary.FindLookAtRotation` _returnvalue _returnvalue_2)) (`KismetMathLibrary.SelectVector` (3.0 0.25 0.1) (1.0 1.0 1.0) (>= (`KismetMathLibrary.VSize` _returnvalue_3) 256.0)))))
          (`SceneComponent.K2_AddLocalRotation` _returnvalue_4 (struct :`Roll` 90.0) false false)
          (`StaticMeshComponent.SetStaticMesh` _returnvalue_4 "/Engine/BasicShapes/Plane.Plane")
          (`PrimitiveComponent.SetMaterial` _returnvalue_4 0 "/Game/Materials/PathMap/MI_Route.MI_Route")
          (`MeshComponent.SetVectorParameterValueOnMaterials` _returnvalue_4 "ColorB" (`KismetMathLibrary.SelectVector` (1.0 1.0 1.0) (0.1 0.1 0.1) (and (== (`local.LocalCurrentX`) (`local.X`)) (== (`local.Z`) (`local.LocalCurrentY`)))))
          (`KismetArrayLibrary.Array_Add` (`self.Pathes`) _returnvalue_4))))))

(fn `UserConstructionScript`
  (locals (Z :type Integer) (X :type Integer) (Connections :type "Array of /Game/BP/Pathmap/PathConnection Structure")))