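; Fuel actor for the planet minigame that orbits a referenced Planet actor, with graph comments that call it an asteroid.
; BeginPlay picks a random orbit speed and randomly flips its sign to set the direction.
; Each Tick rotates the offset from the planet around the world Y axis and applies the difference as an unswept world offset, so only position changes.
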(event `self.ReceiveBeginPlay`
  ;[1 1 1] Seed asteroid speed
  (bind _output_get (set `self.speed` (`KismetMathLibrary.RandomFloatInRange` 8.0 30.0)))
  (if (`KismetMathLibrary.RandomBool`)
    (set `self.speed` _output_get)
    (else
      (set `self.speed` (* _output_get -1.0)))))

(event `self.ReceiveTick`
  (params (DeltaSeconds :type "Float (single-precision)"))
  (bind _returnvalue (- (`self.K2_GetActorLocation`) (`self.K2_GetActorLocation` (`self.planet`))))
  ;[1 1 1] Rotate asteroids around planet
  (`self.K2_AddActorWorldOffset` (- (`KismetMathLibrary.RotateAngleAxis` _returnvalue (* DeltaSeconds (`self.speed`)) (0.0 1.0 0.0)) _returnvalue)))

(fn `UserConstructionScript`)