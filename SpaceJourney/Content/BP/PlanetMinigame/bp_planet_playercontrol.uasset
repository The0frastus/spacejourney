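; Player controller for the planet minigame that loads resources from the game instance and shows the minigame HUD.
; A 30-second timer saves resources and player position to the game instance, then returns to the Overview level.
; Resource edits clamp amounts and broadcast a change event; Hull reaching zero kills the ship pawn and shows the game over widget.
; After game over, Enter starts a new game and reopens Overview.
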(event `CustomEvent_0`
  (bind _asbp_game_instance (cast `/Game/Core/BP_GameInstance` (`GameplayStatics.GetGameInstance`)))
  (`/Game/Core/BP_GameInstance.SaveState` _asbp_game_instance (`self.Resources`) (`/Game/Core/BP_GameInstance.PlayerX` _asbp_game_instance) (`/Game/Core/BP_GameInstance.PlayerY` _asbp_game_instance))
  (`GameplayStatics.OpenLevel` "Overview"))

(event `self.ReceiveBeginPlay`
  (bind _asbp_game_instance (cast `/Game/Core/BP_GameInstance` (`GameplayStatics.GetGameInstance`)))
  (set `self.Resources` (`/Game/Core/BP_GameInstance.Resources` _asbp_game_instance))
  (bind _returnvalue (`|CreateWidget` "/Game/BP/PlanetMinigame/BP_MinigameWidget.BP_MinigameWidget_C" self))
  (bind _output_get (set `self.UI_Widget` _returnvalue))
  (`UserWidget.AddToViewport` _output_get 0)
  (`WidgetBlueprintLibrary.SetInputMode_GameOnly` self)
  (add `self.OnResourceChanged` (delegate `OnResourceChanged_Event_0`))
  (`KismetSystemLibrary.K2_SetTimerDelegate` (delegate `CustomEvent_0`) 30.0))

(event `OnResourceChanged_Event_0` :!signature `self.OnResourceChanged`
  (params (Resource :type "/Game/BP/Events/Resourcen Enum" :default "NewEnumerator0") (NewAmount :type Integer))
  (switch `/Game/BP/Events/Resourcen` Resource
    (:`NewEnumerator0`
      (if (<= NewAmount 0)
        (bind _asp_planet_ship (cast `/Game/BP/PlanetMinigame/p_planet_ship` (`self.K2_GetPawn`)))
        (`/Game/BP/PlanetMinigame/p_planet_ship.PawnDies` _asp_planet_ship)
        (`Widget.RemoveFromParent` (`self.UI_Widget`))
        (bind _returnvalue (`|CreateWidget` "/Game/BP/PlanetMinigame/BP_MiniGameOverWidget.BP_MiniGameOverWidget_C" self))
        (bind _output_get (set `self.UI_GameOver` _returnvalue))
        (`UserWidget.AddToViewport` _output_get 0)
        (set `self.bGameOver` true)))))

(event `Key|Enter`
  (params (Key :type "Key Structure"))
  (:`Pressed`
    (if (`self.bGameOver`)
      (bind _asbp_game_instance (cast `/Game/Core/BP_GameInstance` (`GameplayStatics.GetGameInstance`)))
      (`/Game/Core/BP_GameInstance.StartNewGame` _asbp_game_instance)
      (set `self.bGameOver` false)
      (`GameplayStatics.OpenLevel` "Overview"))))

(fn `GetResource`
  (params (Resource :type "/Game/BP/Events/Resourcen Enum" :default "NewEnumerator0"))
  (returns (Amount :type Integer))
  (for _array_element (`self.Resources`)
    (if (`|EnumEquality` (break `/Game/BP/Pathmap/PlayerResources` _array_element) Resource)
      (return (`.Amount_5_7811A45048D81ACB18AD8785644683AF` (break `/Game/BP/Pathmap/PlayerResources` _array_element)))))
  (return 0))

(fn `ModifyResource`
  (params (Resource :type "/Game/BP/Events/Resourcen Enum" :default "NewEnumerator0") (Amount :type Integer))
  (locals (LocalAmount :type Integer :default 0))
  (for (_array_element _array_index) (`self.Resources`)
    (if (`|EnumEquality` (break `/Game/BP/Pathmap/PlayerResources` _array_element) Resource)
      (bind _output_get (set `local.LocalAmount` (`KismetMathLibrary.Clamp` (+ (`.Amount_5_7811A45048D81ACB18AD8785644683AF` (break `/Game/BP/Pathmap/PlayerResources` _array_element)) Amount) 0 999)))
      (`KismetArrayLibrary.Array_Set` (`self.Resources`) _array_index (make `/Game/BP/Pathmap/PlayerResources` (break `/Game/BP/Pathmap/PlayerResources` _array_element) _output_get (`.Icon_8_63A8BBCA4B5882340FF227B42F64F577` (break `/Game/BP/Pathmap/PlayerResources` _array_element))))
      (`self.OnResourceChanged` (break `/Game/BP/Pathmap/PlayerResources` _array_element) _output_get))))

(fn `UserConstructionScript`)