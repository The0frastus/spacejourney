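; Planet actor for the planet minigame that populates the level with asteroids and fuel pickups and spins continuously.
; On BeginPlay it spawns both at random pitch angles and distances in a zero-yaw plane around the world origin, with fuel in a narrower arc, passing itself as their planet.
; Tick rotates the Planet component around its local pitch axis at YawnPerSecond, despite the variable's name.
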(event `self.ReceiveBeginPlay`
  ;[1 1 1] Spawn asteroid
  (for _ (range 31)
    (bind _asbp_planet_asteroid (castclass `/Game/BP/PlanetMinigame/bp_planet_asteroid` "/Game/BP/PlanetMinigame/bp_planet_asteroid.bp_planet_asteroid_C"))
    (`|SpawnActorFromClass` _asbp_planet_asteroid (`KismetMathLibrary.MakeTransform` (`KismetMathLibrary.CreateVectorFromYawPitch` 0.0 (`KismetMathLibrary.RandomFloatInRange` -160.0 160.0) (`KismetMathLibrary.RandomFloatInRange` 2700.0 4000.0))) "Undefined" "OverrideRootScale" (`ActorComponent.GetOwner` (`self.planet`)) self null))
  ;[1 1 1] Spawn fuel
  (for _ (range 6)
    (bind _asbp_fuel (castclass `/Game/BP/PlanetMinigame/bp_fuel` "/Game/BP/PlanetMinigame/bp_fuel.bp_fuel_C"))
    (`|SpawnActorFromClass` _asbp_fuel (`KismetMathLibrary.MakeTransform` (`KismetMathLibrary.CreateVectorFromYawPitch` 0.0 (`KismetMathLibrary.RandomFloatInRange` -60.0 60.0) (`KismetMathLibrary.RandomFloatInRange` 2500.0 3800.0))) "Undefined" "OverrideRootScale" (`ActorComponent.GetOwner` (`self.planet`)) self null)))

(event `self.ReceiveTick`
  (params (DeltaSeconds :type "Float (single-precision)"))
  ;[1 1 1] Rotate planet
  (`SceneComponent.K2_AddLocalRotation` (`self.planet`) (`KismetMathLibrary.MakeRotator` 0.0 (* DeltaSeconds (`self.yawn per second`))) false false))

(fn `UserConstructionScript`)